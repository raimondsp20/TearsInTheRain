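; MasterWeapon is a weapon Blueprint, apparently the base for pickups, holding a WeaponStruct whose class field the construction script sets to its own class.
; When ThirdPersonCharacter overlaps InteractArea, it sets CanPick and shows a lazily created InteractWidget labeled with the weapon name.
; Hiding the prompt and clearing CanPick runs on the Widget component's hit event, while end overlap is empty.
; Interact only prints a placeholder message.
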(event OnComponentBeginOverlap(InteractArea)
  (params (OverlappedComponent :type Primitive%20Component%20Object%20Reference) (OtherActor :type Actor%20Object%20Reference) (OtherComp :type Primitive%20Component%20Object%20Reference) (OtherBodyIndex :type Integer) (bFromSweep :type Boolean) (SweepResult :type Hit%20Result%20Structure%20%28by%20ref%29))
  (bind _widget (Variables|Default|GetWidget))
  (Utilities|Casting|CastToThirdPersonCharacter OtherActor)
  (Variables|Default|SetCanPick true)
  (Variables|Default|GetInteractUI
    (:then
      _)
    (:else
      (bind _returnvalue (UserInterface|CreateWidget "/Game/Blueprints/InteractWidget.InteractWidget_C" 0 (.WeaponName (Utilities|Struct|BreakWeaStruct (Variables|Default|GetWeaponStruct)))))
      (Variables|Default|SetInteractUI _returnvalue)
      (UserInterface|SetWidget _widget _returnvalue)))
  (Rendering|SetVisibility _widget true false))

(event OnComponentEndOverlap(InteractArea)
  (params (OverlappedComponent :type Primitive%20Component%20Object%20Reference) (OtherActor :type Actor%20Object%20Reference) (OtherComp :type Primitive%20Component%20Object%20Reference) (OtherBodyIndex :type Integer)))

(event OnComponentHit(Widget)
  (params (HitComponent :type Primitive%20Component%20Object%20Reference) (OtherActor :type Actor%20Object%20Reference) (OtherComp :type Primitive%20Component%20Object%20Reference) (NormalImpulse :type Vector :default "0, 0, 0") (Hit :type Hit%20Result%20Structure%20%28by%20ref%29))
  (Rendering|SetVisibility (Variables|Default|GetWidget) false false)
  (Variables|Default|SetCanPick false))

(event EventBeginPlay)

(event Collision|EventActorBeginOverlap
  (params (OtherActor :type Actor%20Object%20Reference)))

(event EventTick
  (params (DeltaSeconds :type Float%20%28single-precision%29)))

(event EventInteract
  (params (Interactor :type Actor%20Object%20Reference))
  (Development|PrintString "Hello"))

(fn ConstructionScript
  (bind _weaponstruct (Variables|Default|GetWeaponStruct))
  (Utilities|Struct|SetmembersinWeaStruct (Variables|Default|GetWeaponStruct) (.weaponname _weaponstruct) (.weaponenumurator _weaponstruct) (Utilities|GetClass self) (.departmentissueammocounter _weaponstruct) (.damage _weaponstruct) (.weaponimage _weaponstruct) (.isameleeweapon _weaponstruct)))